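; MyMath is a math helper with a musical pitch lookup and an integer wrap-around function.
; GetToneMaltiply maps notes C to B to equal-tempered pitch multipliers, with A as 1.0.
; Repeat calls SetupValues to turn Value's position between Min and Max into a wrapped fraction, then returns CalcResoult.
; CalcResoult holds the formula scaling that fraction back into the range, but the expression appears unconnected.
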(fn GetToneMaltiply
  (params (toneCode :type EToneCode%20Enum))
  (return (Utilities|Select :Index toneCode :NewEnumerator0 0.594614 :NewEnumerator1 0.667432 :NewEnumerator2 0.749159 :NewEnumerator3 0.793705 :NewEnumerator4 0.890909 :NewEnumerator5 1.0 :NewEnumerator6 1.122455)))

(fn Repeat
  (params (value :type Integer) (min :type Integer) (max :type Integer))
  (|SetupValues value min max)
  (return (|CalcResoult)))