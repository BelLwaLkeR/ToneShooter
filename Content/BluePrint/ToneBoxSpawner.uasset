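; Spawner actor that builds a ring of seven ToneBox actors on BeginPlay, one per tone.
; Boxes sit at equal angles around the world origin rather than the spawner, facing inward and scaled with the radius.
; Helper functions derive each box's angle, tone enum and color from its index, with phase-shifted sines for RGB.
; The tone lookup also prints a debug string, and octave is left unset.
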(event EventBeginPlay
  (|Make7ToneBox))

(fn ConstructionScript)

(fn SpawnToneBox
  (params (transform :type Transform) (tone :type EToneCode%20Enum) (octave :type Integer) (Color :type Vector))
  (Game|SpawnActorfromClass "/Game/BluePrint/ToneBox.ToneBox_C" transform "AdjustIfPossibleButAlwaysSpawn" 0 tone octave Color))

(fn MakeTransformfromAngle
  (params (angle :type Float%20%28single-precision%29) (radius :type Float%20%28single-precision%29))
  (bind _returnvalue (* radius 0.0048))
  (bind _returnvalue_2 (* _returnvalue 2.0))
  (return (Math|Transform|MakeTransform (+ "0, 0, 0" (* (Math|Vector|GetForwardVector (Math|Rotator|MakeRotator 0.0 0.0 angle)) radius)) (Math|Rotator|MakeRotator 0.0 0.0 (+ angle 1.8e+02)) (Math|Vector|MakeVector 1.0 _returnvalue_2 _returnvalue_2))))

(fn MakeEToneCode
  (params (int :type Integer))
  (bind _resoult (CallFunction|Repeat int 0 7))
  (Development|PrintString (Utilities|String|Append (Utilities|String|Append (Utilities|String|Append "" (Utilities|String|ToString(Integer) int)) " : ") (Utilities|String|ToString(Integer) _resoult)) true true "(R=0.000000,G=0.660000,B=1.000000,A=1.000000)" 6e+01)
  (return (Utilities|Select :Index _resoult :Option%200 "NewEnumerator0" :Option%201 "NewEnumerator1" :Option%202 "NewEnumerator2" :Option%203 "NewEnumerator3" :Option%204 "NewEnumerator4" :Option%205 "NewEnumerator5" :Option%206 "NewEnumerator6")))