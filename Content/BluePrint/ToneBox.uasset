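; ToneBox is a colored box actor that plays a musical tone as a spatialized sound.
; BeginPlay applies BoxColor to the cube's material "Color" parameter.
; PlayTone plays RA_Sound at the actor's location, and AwakeEffect plays it at a supplied position, both with attenuation.
; Both events derive the pitch multiplier from Tone through GetToneMaltiply, so one sample covers different notes.
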(event EventBeginPlay
  (Rendering|Material|SetVectorParameterValueonMaterials (Variables|Default|GetCube) "Color" (Variables|Default|GetBoxColor)))

(event Collision|EventActorBeginOverlap
  (params (OtherActor :type Actor%20Object%20Reference)))

(event EventTick
  (params (DeltaSeconds :type Float%20%28single-precision%29)))

(event EventAwakeEffect
  (params (awakePosition :type Vector))
  (bind _magnification (CallFunction|GetToneMaltiply (Variables|Default|Gettone)))
  (Audio|PlaySoundatLocation "/Game/Sound/RA_Sound.RA_Sound" awakePosition "0.000000, 0, 0" 1.0 _magnification 0.0 "/Game/SoundSoundAttenuation.SoundSoundAttenuation"))

(event EventPlayTone
  (bind _magnification (CallFunction|GetToneMaltiply (Variables|Default|Gettone)))
  (Audio|PlaySoundatLocation "/Game/Sound/RA_Sound.RA_Sound" (Transformation|GetActorLocation) "0.000000, 0, 0" 1.0 _magnification 0.0 "/Game/SoundSoundAttenuation.SoundSoundAttenuation"))

(fn ConstructionScript)