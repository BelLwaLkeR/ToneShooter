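; RhythmBlock is an audio-visualizer actor that updates its Cube's transform from a SoundWave.
; Each Tick, SoundVisualFunction wraps offset game time over the sound's duration and samples a short frequency spectrum there.
; The spectrum feeds MakeBlockTransform, whose result is applied to the Cube with teleport.
; That helper holds math for Z scale from peak amplitude and ImpactScale, though it appears unconnected.
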(event EventBeginPlay)

(event Collision|EventActorBeginOverlap
  (params (OtherActor :type Actor%20Object%20Reference)))

(event EventTick
  (params (DeltaSeconds :type Float%20%28single-precision%29))
  (CallFunction|SoundVisualFunction (Variables|Default|GetSoundWave)))

(fn ConstructionScript)

(fn SoundVisualFunction
  (params (SoundWave :type Sound%20Wave%20Object%20Reference))
  (bind _resoult (CallFunction|Repeatf (- (Utilities|Time|GetGameTimeinSeconds) (Variables|Default|GetTimeOffset)) 0.0 (Variables|/Script/Engine.SoundBase|GetDuration SoundWave)))
  (bind _outspectrum (Class|SoundVisualizationStatics|CalculateFrequencySpectrum SoundWave 0 _resoult 0.01 10))
  (Transformation|SetRelativeTransform (Variables|Default|GetCube) (|MakeBlockTransform _outspectrum) false true))