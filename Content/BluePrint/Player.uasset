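; Player Blueprint that lets the user wake effects on objects by firing from either hand.
; FireL and FireR pass the matching hand's world transform to WakeTone, which runs a debug-drawn Visibility line trace along the hand's forward vector up to ToneWakeRange.
; Hit actors implementing IHitEffectable receive AwakeEffect at the impact location; an older ITonable PlayTone call remains but is disconnected.
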(event Input|ActionEvents|InputActionFireL
  (params (Key :type Key%20Structure :default "AnyKey"))
  (:Pressed
    (CallFunction|WakeTone (Transformation|GetWorldTransform (Variables|Default|GetHandL)))))

(event Input|ActionEvents|InputActionFireR
  (params (Key :type Key%20Structure :default "AnyKey"))
  (:Pressed
    (CallFunction|WakeTone (Transformation|GetWorldTransform (Variables|Default|GetHandR)))))

(fn ConstructionScript)

(fn WakeTone
  (params (handTransform :type Transform))
  (bind (_location _rotation) (Math|Transform|BreakTransform handTransform))
  (bind _outhit (Collision|LineTraceByChannel _location (+ _location (* (Math|Vector|GetForwardVector _rotation) (Variables|Default|GetToneWakeRange))) "TraceTypeQuery1" false 0 "ForDuration" true "(R=1.000000,G=0.000000,B=0.000000,A=1.000000)" "(R=0.000000,G=1.000000,B=0.000000,A=1.000000)" 0.5))
  (bind _asihit_effectable (Utilities|Casting|CastToIHitEffectable (.HitActor (Collision|BreakHitResult _outhit))))
  (Default|AwakeEffect _asihit_effectable (.Location (Collision|BreakHitResult _outhit))))