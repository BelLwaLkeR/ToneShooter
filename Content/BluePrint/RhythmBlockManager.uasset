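; Manager actor that spawns concentric rings of RhythmBlock actors around its own location at BeginPlay and stores them in an array.
; Nested loops scale each ring's radius and block count with its index, rotate it slightly and face blocks outward.
; Each block receives the BGM cue, the center location and an impact scale that weakens outward; time offset evaluates to zero.
; The inclusive inner loop puts a duplicate block at each ring's starting angle.
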(event EventBeginPlay
  (bind _returnvalue (Transformation|GetActorLocation))
  (for _index (range 2 8)
    (for _index_2 (range 0 (Class|KismetSystemLibrary|MakeLiteralInteger (* _index 4)))
      (bind _returnvalue_2 (Game|SpawnActorfromClass "/Game/BluePrint/RhythmBlock.RhythmBlock_C" (Math|Transform|MakeTransform (+ (* (Math|Vector|GetForwardVector (Math|Rotator|MakeRotator 0.0 0.0 (+ (* _index_2 (/ 3.6e+02 (Math|Conversions|ToFloat(Integer) (Class|KismetSystemLibrary|MakeLiteralInteger (* _index 4))))) (* (Math|Conversions|ToFloat(Integer) _index) 5.0)))) (* (Math|Conversions|ToFloat(Integer) _index) 4e+02)) _returnvalue) (Math|Rotator|MakeRotator 0.0 0.0 (+ (* _index_2 (/ 3.6e+02 (Math|Conversions|ToFloat(Integer) (Class|KismetSystemLibrary|MakeLiteralInteger (* _index 4))))) (* (Math|Conversions|ToFloat(Integer) _index) 5.0))) (Math|Vector|MakeVector 3.0 2.0 1.0)) "Undefined" 0 "/Game/Sound/BGM.BGM" (* _index 0.0) (/ 1.0 (* _index 0.1)) _returnvalue))
      (Utilities|Array|Add (Variables|Default|GetRhythmBlocks) _returnvalue_2))))

(fn ConstructionScript)